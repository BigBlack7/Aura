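; BP_SlingshotRock is a rock actor in the enemy abilities folder, named as a slingshot projectile, that tumbles visually.
; BeginPlay picks a random spin rate for each of yaw, pitch and roll, in either direction.
; Tick applies those rates, scaled by delta time, as local rotation on RockMesh for a frame-rate-independent tumble.
; The graph itself contains only this spin logic.
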(event EventBeginPlay
  (bind _returnvalue (Math|Random|RandomFloatinRange -5e+02 5e+02))
  (Variables|Default|SetYaw _returnvalue)
  (Variables|Default|SetPitch _returnvalue)
  (Variables|Default|SetRoll _returnvalue))

(event EventTick
  (params (DeltaSeconds :type Float%20%28single-precision%29))
  (Transformation|AddLocalRotation (Variables|Default|GetRockMesh) (Math|Rotator|MakeRotator (* DeltaSeconds (Variables|Default|GetRoll)) (* DeltaSeconds (Variables|Default|GetPitch)) (* DeltaSeconds (Variables|Default|GetYaw))) false false))

(fn ConstructionScript)